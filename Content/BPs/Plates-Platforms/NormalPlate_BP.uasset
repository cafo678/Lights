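; NormalPlate_BP is a pressure plate that swings a door or rotates a slide, depending on the class of its ControlledActor.
; Overlapping its collision volume changes the plate color and fires Activate or Disactivate; Utilized is set on first contact and never cleared here.
; A RotatSlide_BP target follows a pitch timeline that stops in place on release.
; Other actors follow a yaw timeline, offset from their BeginPlay angle, that reverses on release.
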(event OnComponentBeginOverlap(CollisionVolume)
  (params (OverlappedComponent :type Primitive%20Component%20Object%20Reference) (OtherActor :type Actor%20Object%20Reference) (OtherComp :type Primitive%20Component%20Object%20Reference) (OtherBodyIndex :type Integer) (bFromSweep :type Boolean) (SweepResult :type Hit%20Result%20Structure%20%28by%20ref%29))
  ;[1 1 1] On Begin/End Overlap change the color, set bUtilized and fire the events
  (Variables|Default|SetbUtilized true)
  (Class|Plate|ChangePlateColor)
  (CallFunction|Activate))

(event OnComponentEndOverlap(CollisionVolume)
  (params (OverlappedComponent :type Primitive%20Component%20Object%20Reference) (OtherActor :type Actor%20Object%20Reference) (OtherComp :type Primitive%20Component%20Object%20Reference) (OtherBodyIndex :type Integer))
  ;[1 1 1] On Begin/End Overlap change the color, set bUtilized and fire the events
  (Class|Plate|ChangePlateColor)
  (CallFunction|Disactivate))

(event Custom|Activate
  (bind _controlledactor (Variables|Default|GetControlledActor))
  (bind _returnvalue (Transformation|GetActorRotation _controlledactor))
  ;[1 1 1] Events with timelines for Open Door or Rotate the Slides based on the class of the Controlled Actor
  (if (Utilities|ClassIsChildOf (Utilities|GetClass (Variables|Default|GetControlledActor)) "/Game/BPs/Plates-Platforms/RotatSlide_BP.RotatSlide_BP_C")
    (bind _newysliderotation (Timeline|RotatSlide%20Rotation Play)
      (:Update
        (Transformation|SetActorRotation (Variables|Default|GetControlledActor) (Math|Rotator|MakeRotator (Math|Float|Clamp(Float) (.roll _returnvalue) 0.0 359.899994) (Math|Float|Clamp(Float) _newysliderotation 0.0 359.899994) (Math|Float|Clamp(Float) (.yaw _returnvalue) 0.0 359.899994)))))
    (else
      (bind _newzdoorrotation (Timeline|Door%20Swing Play)
        (:Update
          (Transformation|SetActorRotation (Variables|Default|GetControlledActor) (Math|Rotator|MakeRotator 0.0 0.0 (+ _newzdoorrotation (Variables|Default|GetDoorInitialAngle)))))))))

(event Custom|Disactivate
  (bind _controlledactor (Variables|Default|GetControlledActor))
  (bind _returnvalue (Transformation|GetActorRotation _controlledactor))
  ;[1 1 1] Events with timelines for Open Door or Rotate the Slides based on the class of the Controlled Actor
  (if (Utilities|ClassIsChildOf (Utilities|GetClass (Variables|Default|GetControlledActor)) "/Game/BPs/Plates-Platforms/RotatSlide_BP.RotatSlide_BP_C")
    (bind _newysliderotation (Timeline|RotatSlide%20Rotation Stop)
      (:Update
        (Transformation|SetActorRotation (Variables|Default|GetControlledActor) (Math|Rotator|MakeRotator (Math|Float|Clamp(Float) (.roll _returnvalue) 0.0 359.899994) (Math|Float|Clamp(Float) _newysliderotation 0.0 359.899994) (Math|Float|Clamp(Float) (.yaw _returnvalue) 0.0 359.899994)))))
    (else
      (bind _newzdoorrotation (Timeline|Door%20Swing Reverse)
        (:Update
          (Transformation|SetActorRotation (Variables|Default|GetControlledActor) (Math|Rotator|MakeRotator 0.0 0.0 (+ _newzdoorrotation (Variables|Default|GetDoorInitialAngle)))))))))

(event EventBeginPlay
  ;[1 1 1] Set Door Initial Angle on BeginPlay
  (|CallParentFunction)
  (Variables|Default|SetDoorInitialAngle (.yaw (Transformation|GetWorldRotation (Variables|/Script/Engine.Actor|GetRootComponent (Variables|Default|GetControlledActor))))))

(fn ConstructionScript)