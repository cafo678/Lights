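; SlidePlate_BP is a color-coded trigger plate that removes matching SlidePlatform_BP platforms while overlapped.
; On begin overlap of its CollisionVolume it calls ChangePlateColor, then hides and disables collision on every platform whose PlatformColor equals its PlateColor.
; End overlap calls ChangePlateColor again and restores those platforms.
; Both events search the level with GetAllActorsOfClass and do not filter the overlapping actor.
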(event OnComponentBeginOverlap(CollisionVolume)
  (params (OverlappedComponent :type Primitive%20Component%20Object%20Reference) (OtherActor :type Actor%20Object%20Reference) (OtherComp :type Primitive%20Component%20Object%20Reference) (OtherBodyIndex :type Integer) (bFromSweep :type Boolean) (SweepResult :type Hit%20Result%20Structure%20%28by%20ref%29))
  ;[1 1 1] On Begin/End Overlap change the color, find all the platform of the same color and hide them
  (Class|Plate|ChangePlateColor)
  (bind _outactors (Actor|GetAllActorsOfClass "/Game/BPs/Plates-Platforms/SlidePlatform_BP.SlidePlatform_BP_C"))
  (for _array_element _outactors
    (if (== (Variables|/Script/Lights.SlidePlatform|GetPlatformColor _array_element) (Variables|Default|GetPlateColor))
      (Rendering|SetActorHiddenInGame _array_element true)
      (Collision|SetActorEnableCollision _array_element false))))

(event OnComponentEndOverlap(CollisionVolume)
  (params (OverlappedComponent :type Primitive%20Component%20Object%20Reference) (OtherActor :type Actor%20Object%20Reference) (OtherComp :type Primitive%20Component%20Object%20Reference) (OtherBodyIndex :type Integer))
  ;[1 1 1] On Begin/End Overlap change the color, find all the platform of the same color and hide them
  (Class|Plate|ChangePlateColor)
  (bind _outactors (Actor|GetAllActorsOfClass "/Game/BPs/Plates-Platforms/SlidePlatform_BP.SlidePlatform_BP_C"))
  (for _array_element _outactors
    (if (== (Variables|/Script/Lights.SlidePlatform|GetPlatformColor _array_element) (Variables|Default|GetPlateColor))
      (Rendering|SetActorHiddenInGame _array_element false)
      (Collision|SetActorEnableCollision _array_element true))))

(fn ConstructionScript)