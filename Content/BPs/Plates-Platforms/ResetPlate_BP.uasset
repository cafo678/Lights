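; Pressure plate that resets a puzzle sphere when the player's pawn steps on it.
; Overlap moves the sphere to its reset location, zeroes its linear physics velocity and calls ResetEvent on the linked TelePlate if one is valid.
; The plate changes color when the player enters and again when any overlap ends, since the end event does not filter by actor.
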(event OnComponentBeginOverlap(CollisionVolume)
  (params (OverlappedComponent :type Primitive%20Component%20Object%20Reference) (OtherActor :type Actor%20Object%20Reference) (OtherComp :type Primitive%20Component%20Object%20Reference) (OtherBodyIndex :type Integer) (bFromSweep :type Boolean) (SweepResult :type Hit%20Result%20Structure%20%28by%20ref%29))
  (bind _teleplateref (Variables|Default|GetTelePlateRef))
  ;[1 1 1] Comment
  (if (== OtherActor (Game|Player|GetPlayerPawn 0))
    (Class|Plate|ChangePlateColor)
    (Transformation|SetActorLocation (Variables|Default|GetSphere) (Variables|Default|GetSphereResetLocation) false false)
    (Class|PrimitiveComponent|SetAllPhysicsLinearVelocity (Actor|GetComponentbyClass (Variables|Default|GetSphere) "/Script/Engine.PrimitiveComponent") "0, 0, 0" false)
    (if (Utilities|IsValid _teleplateref)
      (Default|ResetEvent _teleplateref))))

(event OnComponentEndOverlap(CollisionVolume)
  (params (OverlappedComponent :type Primitive%20Component%20Object%20Reference) (OtherActor :type Actor%20Object%20Reference) (OtherComp :type Primitive%20Component%20Object%20Reference) (OtherBodyIndex :type Integer))
  ;[1 1 1] Comment
  (Class|Plate|ChangePlateColor))

(fn ConstructionScript)