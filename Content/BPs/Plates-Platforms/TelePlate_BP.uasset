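; TelePlate is a plate Blueprint, apparently for teleporting, that starts a plate selection when the player pawn overlaps its collision volume.
; A DoOnce gates the overlap, which gathers valid plates from TrigList and then sets up the selection.
; Reset_Event re-arms the gate and restores the old command widget text when that widget is valid.
; The QuitSelection input also re-arms the gate after a short delay.
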(event OnComponentBeginOverlap(CollisionVolume)
  (params (OverlappedComponent :type Primitive%20Component%20Object%20Reference) (OtherActor :type Actor%20Object%20Reference) (OtherComp :type Primitive%20Component%20Object%20Reference) (OtherBodyIndex :type Integer) (bFromSweep :type Boolean) (SweepResult :type Hit%20Result%20Structure%20%28by%20ref%29))
  ;[1 1 1] On BeginOverlap get the valid plates and setup the plate selection
  (if (== OtherActor (Game|Player|GetPlayerPawn 0))
    (Utilities|FlowControl|DoOnce false
      (:Completed
        (Class|TelePlate|GetValidPlates (Variables|Default|GetTrigList))
        (Class|TelePlate|SetupPlateSelection)))))

(event Custom|Reset_Event
  ;[1 1 1] Events that reset the DoOnce of the TelePlate and change the command list
  (if (Utilities|IsValid (Variables|Default|GetCommandTextWidget))
    (Rendering|Components|TextRender|SetText (Variables|/Script/Lights.CommandTextWidget|GetCommandText (Variables|Default|GetCommandTextWidget)) (Variables|Default|GetOldWidgetText))
    ;[1 1 1] On BeginOverlap get the valid plates and setup the plate selection
    (Utilities|FlowControl|DoOnce false) ; enters at Reset
    (else
      (Utilities|FlowControl|DoOnce false) ; enters at Reset
    )))

(event Input|ActionEvents|InputActionQuitSelection
  (params (Key :type Key%20Structure :default "None"))
  ;[1 1 1] Events that reset the DoOnce of the TelePlate and change the command list
  (:Pressed
    (Utilities|FlowControl|Delay 2.0)
    ;[1 1 1] On BeginOverlap get the valid plates and setup the plate selection
    (Utilities|FlowControl|DoOnce false) ; enters at Reset
  ))

(fn ConstructionScript)